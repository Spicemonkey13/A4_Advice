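; Player character for melee combat, with movement, directional jump montages, stamina-limited sprinting and a HUD.
; Combo attacks soft-target living, unobstructed enemies by camera angle and proximity to a point ahead, then feed Motion Warping.
; Damage updates the stats component, turns the player toward the causer, cancels the combo and temporarily removes combat input.
; BeginPlay restores transform, stats and equipped weapon from the GameInstance, with weapons held in a child actor.
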(event `self.OnJumped`
  (`self.PlayDirectionalJumpAnim`))

(event `self.OnLanded`
  (params (Hit :type "HitResult Structure (by ref)"))
  (`self.PlayAnimMontage` (`self.LandAnim`)))

(event `LerpActorToControlRotation`
  (params (Duration :type "Float (double-precision)" :default 0.25))
  (bind (_returnvalue_roll _returnvalue_pitch _returnvalue_yaw) (`KismetMathLibrary.BreakRotator` (`self.GetControlRotation`)))
  (`self.K2_SetActorRotation` (`KismetMathLibrary.MakeRotator` 0.0 0.0 _returnvalue_yaw)))

(event `self.ReceiveAnyDamage`
  (params (Damage :type "Float (single-precision)") (DamageType :type "DamageType Object Reference") (InstigatedBy :type "Controller Object Reference") (DamageCauser :type "Actor Object Reference"))
  (bind (_returnvalue_roll _returnvalue_pitch _returnvalue_yaw) (`KismetMathLibrary.BreakRotator` (`KismetMathLibrary.FindLookAtRotation` (`self.K2_GetActorLocation`) (`self.K2_GetActorLocation` DamageCauser))))
  (`/Game/MyContent/Core/BP_AC_Stats.DamageHealth` (`self.Stats Component (Player)`) Damage)
  (`self.K2_SetActorRotation` (`KismetMathLibrary.MakeRotator` 0.0 0.0 _returnvalue_yaw))
  (`self.PlayerHitReact`)
  (bind _asbp_player_controller (cast `/Game/MyContent/Player/BP_PlayerController` (`self.GetController`)))
  (`/Game/MyContent/Player/BP_PlayerController.DisableGameMenu` _asbp_player_controller))

(event `InputAction|Sprint`
  (params (Key :type "Key Structure"))
  ;[1 1 1] Sprint
  (:`Pressed`
    (`self.StartSprinting`))
  (:`Released`
    (`self.StopSprinting`)))

(event `Drain Stamina`
  (bind _output_get (set `self.Stamina` (`KismetMathLibrary.Clamp` (- (`self.Stamina`) 1) 0 (`self.MaxStamina`))))
  (if (== _output_get 0)
    (`self.StopSprinting`)
    (elif (`self.IsSprinting?`)
      (`KismetSystemLibrary.Delay` 0.1)
      (`self.Drain Stamina`))))

(event `Regain Stamina`
  (bind _output_get (set `self.Stamina` (`KismetMathLibrary.Clamp` (+ (`self.Stamina`) 5) 0 (`self.MaxStamina`))))
  (if (== _output_get (`self.MaxStamina`))
    _
    (elif (not (`self.IsSprinting?`))
      (`KismetSystemLibrary.Delay` 0.05)
      (`self.Regain Stamina`))))

(event `self.ReceiveBeginPlay`
  (`self.LoadSavedData`)
  (bind _returnvalue (`|CreateWidget` "/Game/MyContent/Player/HUD/BP_UI_Player_HUD.BP_UI_Player_HUD_C"))
  (`UserWidget.AddToViewport` _returnvalue 0))

(fn `ActivateWeaponDamage`
  (bind _asbp_weapon (cast `/Game/MyContent/Items/BP_Weapon` (`ChildActorComponent.ChildActor` (`self.WeaponActorComponent`))))
  (`/Game/MyContent/Items/BP_Weapon.ActivateDamage` _asbp_weapon))

(fn `AddInput`
  (params (MappingContext :type "InputMappingContext Object Reference") (Priority :type Integer) (` Ignore All Pressed Keys Until Release` :type Boolean :default true))
  (bind _asbp_player_controller (cast `/Game/MyContent/Player/BP_PlayerController` (`GameplayStatics.GetPlayerController` 0)))
  (`/Game/MyContent/Player/BP_PlayerController.AddInput` _asbp_player_controller MappingContext Priority ` Ignore All Pressed Keys Until Release`))

(fn `AllowNextCombo`
  (set `self.IsNextComboAllowed` true))

(fn `BasicComboAttack`
  (locals (LTestTarget :type "Actor Object Reference"))
  (if (and (`self.IsNextComboAllowed`) (not (`NavMovementComponent.IsFalling` (`self.CharacterMovement`))))
    (set `self.IsNextComboAllowed` false)
    (bind _actor (`self.Find Attack Target`))
    (bind _output_get (set `local.LTestTarget` _actor))
    (`self.SetWarpTarget` _output_get)
    (`self.PlayReleventComboAnim`)
    (`self.IncrementComboCounter`)
    (if (not (`KismetSystemLibrary.IsValid` (`local.LTestTarget`)))
      (`self.LerpActorToControlRotation` 0.2))))

(fn `CompareTargetAngle`
  (params (PotentialTargets :type "Array of Actor Object Reference") (Debug :type Boolean))
  (returns (TargetsWithinAngle :type "Array of Actor Object Reference") (Success :type Boolean))
  (locals (LTestTarget :type "Actor Object Reference") (LTargetsWithAngle :type "Array of Actor Object Reference") (SoftTargetAngle :type "Float (double-precision)" :default 0.2))
  (bind (_returnvalue_roll _returnvalue_pitch _returnvalue_yaw) (`KismetMathLibrary.BreakRotator` (`self.GetControlRotation`)))
  (bind _ltesttarget (`local.LTestTarget`))
  (bind (_origin _boxextent) (`self.GetActorBounds` _ltesttarget true false))
  (bind (_returnvalue_roll_2 _returnvalue_pitch_2 _returnvalue_yaw_2) (`KismetMathLibrary.BreakRotator` (`KismetMathLibrary.FindLookAtRotation` (`self.K2_GetActorLocation`) (`self.K2_GetActorLocation` (`local.LTestTarget`)))))
  (for _array_element PotentialTargets
    (set `local.LTestTarget` _array_element)
    (if (>= (`KismetMathLibrary.Dot_VectorVector` (`KismetMathLibrary.GetForwardVector` (`KismetMathLibrary.MakeRotator` 0.0 0.0 _returnvalue_yaw_2)) (`KismetMathLibrary.GetForwardVector` (`KismetMathLibrary.MakeRotator` 0.0 0.0 _returnvalue_yaw))) (`local.SoftTargetAngle`))
      (`KismetArrayLibrary.Array_Add` (`local.LTargetsWithAngle`) (`local.LTestTarget`))
      (if (`local.Debug`)
        (`KismetSystemLibrary.DrawDebugBox` _origin _boxextent (struct :`R` 1.0 :`G` 0.793775 :`B` 0.034391 :`A` 1.0) (`self.K2_GetActorRotation` _ltesttarget) 5.0))))
  (return (`local.LTargetsWithAngle`) (`KismetArrayLibrary.Array_IsNotEmpty` (`local.LTargetsWithAngle`))))

(fn `ControlCamera`
  (params (Axis :type "Vector2D Structure"))
  (`|ExecutionSequence`
    (:`then_0`
      (`self.AddControllerYawInput` Axis_X))
    (:`then_1`
      (`self.AddControllerPitchInput` Axis_Y))))

(fn `DeactivateWeaponDamage`
  (bind _asbp_weapon (cast `/Game/MyContent/Items/BP_Weapon` (`ChildActorComponent.ChildActor` (`self.WeaponActorComponent`))))
  (`/Game/MyContent/Items/BP_Weapon.DeactivateDamage` _asbp_weapon))

(fn `DetectPotentialTarget`
  (params (Debug :type Boolean))
  (returns (PotentialTargets :type "Array of Actor Object Reference") (bSuccess :type Boolean))
  (locals (LTestTarget :type "Actor Object Reference") (LPotentialTargets :type "Array of Actor Object Reference"))
  (bind (_outradius _outhalfheight) (`CapsuleComponent.GetScaledCapsuleSize` (`self.CapsuleComponent`)))
  (`|ExecutionSequence`
    (:`then_0`
      (if (`local.Debug`)
        (`KismetSystemLibrary.DrawDebugSphere` (`self.K2_GetActorLocation`) (`self.MeleeAttackRange`) 12 (struct :`R` 1.0 :`A` 1.0) 5.0)))
    (:`then_1`
      (bind _outactors (`KismetSystemLibrary.SphereOverlapActors` (`self.K2_GetActorLocation`) (`self.MeleeAttackRange`) (`self.TargetObjectTypes`) null (`|MakeArray` self :!type "Actor Object Reference")))
      (for _array_element _outactors
        (set `local.LTestTarget` _array_element)
        (bind _returnvalue (`self.GetComponentByClass` _array_element "/Game/MyContent/Core/BP_AC_Stats.BP_AC_Stats_C"))
        (`/Engine/EditorBlueprintResources/StandardMacros.IsValid` _returnvalue
          (:`Is Valid`
            (if (`/Game/MyContent/Core/BP_AC_Stats.IsAlive` _returnvalue)
              (bind (_outhit _returnvalue_2) (`KismetSystemLibrary.CapsuleTraceSingleForObjects` :`Start` (`self.K2_GetActorLocation`) :`End` (`self.K2_GetActorLocation` (`local.LTestTarget`)) :`Radius` (* _outradius 0.5) :`HalfHeight` (* _outhalfheight 0.9) :`ObjectTypes` (`|MakeArray` "ObjectTypeQuery1" :!type "EObjectTypeQuery Enum") :`DrawDebugType` (select `bool` (`local.Debug`) :`true` "ForDuration" :!type "EDrawDebugTrace Enum")))
              (if (not _returnvalue_2)
                (`KismetArrayLibrary.Array_Add` (`local.LPotentialTargets`) (`local.LTestTarget`)))))))
      (return (`local.LPotentialTargets`) (`KismetArrayLibrary.Array_IsNotEmpty` (`local.LPotentialTargets`))))))

(fn `DisableAttack`
  (params (Duration :type "Float (double-precision)"))
  (`self.RemoveInput` "/Game/MyContent/Player/Input/IMC_Combat.IMC_Combat")
  (bind _returnvalue (`KismetSystemLibrary.K2_SetTimerDelegate` (`|CreateDelegate` :!event `EnableAttack`) Duration))
  (set `self.TH_EnableAttack` _returnvalue))

(fn `EnableAttack`
  (`self.AddInput` "/Game/MyContent/Player/Input/IMC_Combat.IMC_Combat")
  (`KismetSystemLibrary.K2_ClearAndInvalidateTimerHandle` (`self.TH_EnableAttack`)))

(fn `Find Attack Target`
  (returns (Actor :type "Actor Object Reference"))
  (`KismetSystemLibrary.FlushPersistentDebugLines`)
  (bind (_potentialtargets _bsuccess) (`self.DetectPotentialTarget` true))
  (if _bsuccess
    (bind (_targetswithinangle _success) (`self.CompareTargetAngle` _potentialtargets))
    (if _success
      (bind _closestactor (`self.FindTargetClosestToSelf` _targetswithinangle))
      (return _closestactor)
      (else
        (return null)))
    (else
      (return null))))

(fn `FindTargetClosestToSelf`
  (params (Actors :type "Array of Actor Object Reference") (Debug :type Boolean))
  (returns (ClosestActor :type "Actor Object Reference"))
  (locals (LTestTarget :type "Actor Object Reference") (LClosestActor :type "Actor Object Reference") (LClosestDistance :type "Float (double-precision)") (SoftTargetDistance :type "Float (double-precision)" :default 1.0))
  (for (_array_element _array_index) Actors
    (set `local.LTestTarget` _array_element)
    (if (or (== _array_index 0) (< (`KismetMathLibrary.Vector_DistanceSquared` (`self.K2_GetActorLocation` (`local.LTestTarget`)) (`self.GetLocFromActorBasedOnControl` (`local.SoftTargetDistance`))) (`local.LClosestDistance`)))
      (set `local.LClosestActor` (`local.LTestTarget`))
      (set `local.LClosestDistance` (`KismetMathLibrary.Vector_DistanceSquared` (`self.K2_GetActorLocation` (`local.LTestTarget`)) (`self.GetLocFromActorBasedOnControl` (`local.SoftTargetDistance`))))))
  (`|ExecutionSequence`
    (:`then_0`
      (if (`local.Debug`)
        (`KismetSystemLibrary.DrawDebugSphere` (`self.K2_GetActorLocation` (`local.LClosestActor`)) 30.0 12 (struct :`R` 0.023906 :`G` 1.0 :`B` 0.00239 :`A` 1.0) 5.0)
        (`KismetSystemLibrary.DrawDebugArrow` (`self.K2_GetActorLocation`) (`self.GetLocFromActorBasedOnControl` (`local.SoftTargetDistance`)) 2000.0 (struct :`G` 0.110355 :`B` 1.0 :`A` 1.0) 5.0)))
    (:`then_1`
      (return (`local.LClosestActor`)))))

(fn `ForceCancelBasicAttack`
  (`self.AllowNextCombo`)
  (`self.ResetCombo`))

(fn `GetActorDirection`
  (returns (ReturnValue :type "Float (single-precision)"))
  (return (`KismetAnimationLibrary.CalculateDirection` (`self.GetVelocity`) (`self.K2_GetActorRotation`))))

(fn `GetLocFromActorBasedOnControl`
  (params (Distance :type "Float (double-precision)" :default 1.0))
  (returns (ReturnValue :type "Vector Structure"))
  (bind (_returnvalue_roll _returnvalue_pitch _returnvalue_yaw) (`KismetMathLibrary.BreakRotator` (`self.GetControlRotation`)))
  (return (+ (`self.K2_GetActorLocation`) (* (`KismetMathLibrary.GetForwardVector` (`KismetMathLibrary.MakeRotator` 0.0 0.0 _returnvalue_yaw)) Distance))))

(fn `IncrementComboCounter`
  (bind _result (`/Engine/EditorBlueprintResources/StandardMacros.IncrementInt` (`self.Combo`))
    (:`  `
      (if (not (`KismetArrayLibrary.Array_IsValidIndex` (`self.BasicAttackComboAnims`) _result))
        (set `self.Combo` 0)))))

(fn `InitialiseWeapon`
  (params (Weapon :type "/Game/MyContent/Items/BP_Weapon Class Reference"))
  (`ChildActorComponent.SetChildActorClass` (`self.WeaponActorComponent`) Weapon)
  (`self.SetOwner` (`ChildActorComponent.ChildActor` (`self.WeaponActorComponent`)) self))

(fn `Is Actor Direction Between`
  (params (Min :type "Float (double-precision)") (Max :type "Float (double-precision)"))
  (returns (ReturnValue :type Boolean))
  (bind _returnvalue (`self.GetActorDirection`))
  (return (and (>= _returnvalue Min) (<= _returnvalue Max))))

(fn `LoadSavedData`
  (locals (LGameInstanceRef :type "/Game/MyContent/Core/BP_GameInstance Object Reference") (LSaveGame :type "/Game/MyContent/SaveGame/BP_SaveGame Object Reference"))
  (bind _asbp_game_instance (cast `/Game/MyContent/Core/BP_GameInstance` (`GameplayStatics.GetGameInstance`)))
  (set `local.LGameInstanceRef` _asbp_game_instance)
  (`|ExecutionSequence`
    (:`then_0`
      (bind _savedgame (`/Game/MyContent/Core/BP_GameInstance.SavedGame` (`local.LGameInstanceRef`))
        (:`then`
          (bind _output_get (set `local.LSaveGame` _savedgame))
          (bind _playertransform (`/Game/MyContent/SaveGame/BP_SaveGame.PlayerTransform` _output_get))
          (`self.K2_SetActorTransform` _playertransform false true)
          (`Controller.SetControlRotation` (`self.GetController`) (.rotation _playertransform))
          (`self.TryLevelUp` (`/Game/MyContent/SaveGame/BP_SaveGame.Level` (`local.LSaveGame`)))
          (`/Game/MyContent/Core/BP_AC_Stats.Set Health` (`self.Stats Component (Player)`) (`/Game/MyContent/SaveGame/BP_SaveGame.Health` (`local.LSaveGame`)))
          (`/Game/MyContent/Core/BP_AC_Stats_Player.SetXP` (`self.Stats Component (Player)`) (`/Game/MyContent/SaveGame/BP_SaveGame.XP` (`local.LSaveGame`))))
        (:`else`)))
    (:`then_1`
      (bind _asbp_weapon (castclass `/Game/MyContent/Items/BP_Weapon` (`.Class_2_40A8B29345CB72F60235568B185E765E` (break `/Game/MyContent/Items/ST_InventoryItem` (`/Game/MyContent/Core/BP_GameInstance.EquippedWeapon` _asbp_game_instance)))))
      (`self.InitialiseWeapon` _asbp_weapon))))

(fn `MoveCharacter`
  (params (Axis :type "Vector2D Structure"))
  (bind (_returnvalue_roll _returnvalue_pitch _returnvalue_yaw) (`KismetMathLibrary.BreakRotator` (`self.GetControlRotation`)))
  (bind (_x _y) (`KismetMathLibrary.BreakVector2D` Axis))
  (bind _returnvalue (`KismetMathLibrary.MakeRotator` 0.0 0.0 _returnvalue_yaw))
  (`|ExecutionSequence`
    (:`then_0`
      (`self.AddMovementInput` (`KismetMathLibrary.GetRightVector` _returnvalue) _x))
    (:`then_1`
      (`self.AddMovementInput` (`KismetMathLibrary.GetForwardVector` _returnvalue) _y))
    (:`then_2`
      (set `CharacterMovementComponent.bOrientRotationToMovement` (<= (`KismetMathLibrary.VSize2DSquared` Axis) 0.0) (`self.CharacterMovement`)))))

(fn `PlayDirectionalJumpAnim`
  (if (or (`self.Is Actor Direction Between` -45.0 45.0) (<= (`KismetMathLibrary.VSizeXY` (`self.GetVelocity`)) 0.0))
    (`self.PlayAnimMontage` (`self.JumpForwardAnim`))
    (elif (`self.Is Actor Direction Between` 45.0 125.0)
      (`self.PlayAnimMontage` (`self.JumpRightAnim`))
      (elif (`self.Is Actor Direction Between` -125.0 -45.0)
        (`self.PlayAnimMontage` (`self.JumpLeftAnim`))
        (else
          (`self.PlayAnimMontage` (`self.JumpBackAnim`)))))))

(fn `PlayerHitReact`
  (bind _returnvalue (`AnimInstance.Montage_Play` (`SkeletalMeshComponent.GetAnimInstance` (`self.Mesh`)) "/Game/MyContent/Player/Anim/Seq2/08_Hit/06_Hit_Large_Combat/Player_Hit_Large_Combat_F_Seq_Montage.Player_Hit_Large_Combat_F_Seq_Montage" 1.0 "MontageLength" 0.0 true))
  (`self.DisableAttack` (/ _returnvalue 2.0))
  (`self.DeactivateWeaponDamage`)
  (`self.ForceCancelBasicAttack`))

(fn `PlayReleventComboAnim`
  (if (`KismetArrayLibrary.Array_IsValidIndex` (`self.BasicAttackComboAnims`) (`self.Combo`))
    (`AnimInstance.Montage_Play` (`SkeletalMeshComponent.GetAnimInstance` (`self.Mesh`)) (`|GetArrayItem` (`self.BasicAttackComboAnims`) (`self.Combo`)) 1.0 "MontageLength" 0.0 true)))

(fn `RemoveInput`
  (params (MappingContext :type "InputMappingContext Object Reference") (`Ignore All Pressed Keys Until Release` :type Boolean :default true))
  (bind _asbp_player_controller (cast `/Game/MyContent/Player/BP_PlayerController` (`GameplayStatics.GetPlayerController` 0)))
  (`/Game/MyContent/Player/BP_PlayerController.RemoveInput` _asbp_player_controller MappingContext `Ignore All Pressed Keys Until Release`))

(fn `ResetCombo`
  (set `self.Combo` 0))

(fn `SetWarpTarget`
  (params (TargetActor :type "Actor Object Reference"))
  (bind (_returnvalue_roll _returnvalue_pitch _returnvalue_yaw) (`KismetMathLibrary.BreakRotator` (`KismetMathLibrary.FindLookAtRotation` (`self.K2_GetActorLocation`) (`self.K2_GetActorLocation` (`local.TargetActor`)))))
  (`/Engine/EditorBlueprintResources/StandardMacros.IsValid` TargetActor
    (:`Is Valid`
      (`MotionWarpingComponent.AddOrUpdateWarpTargetFromLocationAndRotation` (`self.MotionWarping`) "BasicAttackTarget" (`self.K2_GetActorLocation` (`local.TargetActor`)) (`KismetMathLibrary.MakeRotator` 0.0 0.0 _returnvalue_yaw)))
    (:`Is Not Valid`
      (`MotionWarpingComponent.RemoveWarpTarget` (`self.MotionWarping`) "BasicAttackTarget"))))

(fn `StartSprinting`
  (set `CharacterMovementComponent.MaxWalkSpeed` 900.0 (`self.CharacterMovement`))
  (set `self.IsSprinting?` true)
  (`self.Drain Stamina`))

(fn `StopSprinting`
  (set `CharacterMovementComponent.MaxWalkSpeed` 600.0 (`self.CharacterMovement`))
  (set `self.IsSprinting?` false)
  (`self.Regain Stamina`))

(fn `TryJump`
  (params (`Pressed/Released` :type Boolean))
  (if (`self.IsNextComboAllowed`)
    (if `Pressed/Released`
      (`self.Jump`)
      (else
        (`self.StopJumping`)))))

(fn `TryLevelUp`
  (params (Level :type "Float (double-precision)"))
  (`/Game/MyContent/Core/BP_AC_Stats.SetLevel` (`self.Stats Component (Player)`) Level))

(fn `UserConstructionScript`
  (`self.InitialiseWeapon` "/Game/MyContent/Items/BP_Weapon_DarkKnight.BP_Weapon_DarkKnight_C"))