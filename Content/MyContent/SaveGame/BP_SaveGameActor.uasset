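; BP_SaveGameActor is a checkpoint actor that saves the game when the player character enters its collision volume.
; On overlap it checks the game instance's saved game and skips saving if this actor is already the recorded save point.
; Otherwise it calls CreateSaveGame on BP_GameInstance, passing the PlayerSpawn component's world transform and its own object name as the save ID.
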(event `self.SaveCollison.OnComponentBeginOverlap`
  (params (OverlappedComponent :type "PrimitiveComponent Object Reference") (OtherActor :type "Actor Object Reference") (OtherComp :type "PrimitiveComponent Object Reference") (OtherBodyIndex :type Integer) (bFromSweep :type Boolean) (SweepResult :type "HitResult Structure (by ref)"))
  (cast `/Game/MyContent/Player/BP_PlayerCharacter` OtherActor)
  (bind _asbp_game_instance (cast `/Game/MyContent/Core/BP_GameInstance` (`GameplayStatics.GetGameInstance`)))
  (if (not (`KismetStringLibrary.EqualEqual_StrStr` (`/Game/MyContent/SaveGame/BP_SaveGame.SaveActorID` (`/Game/MyContent/Core/BP_GameInstance.SavedGame` _asbp_game_instance)) (`KismetSystemLibrary.GetObjectName` self)))
    (`self.SaveGame`)))

(fn `SaveGame`
  (bind _asbp_game_instance (cast `/Game/MyContent/Core/BP_GameInstance` (`GameplayStatics.GetGameInstance`)))
  (`/Game/MyContent/Core/BP_GameInstance.CreateSaveGame` _asbp_game_instance (`SceneComponent.K2_GetComponentToWorld` (`self.PlayerSpawn`)) (`KismetSystemLibrary.GetObjectName` self)))

(fn `UserConstructionScript`)